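; Throwable grenade actor for the shooting range that explodes on a fuse after its ThrowedGrenade event is called.
; Detonation plays sound and particle effects at the mesh, hides it and schedules the actor's removal.
; A sphere trace against PhysicsBody objects, with debug drawing left on, applies damage per hit and pushes simulating components away from the blast center.
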(event Custom|ThrowedGrenade
  (bind _staticmesh (Variables|Default|GetStaticMesh))
  (bind _returnvalue (Transformation|GetWorldLocation _staticmesh))
  (Utilities|FlowControl|Delay 1.5)
  (Audio|PlaySoundatLocation "/Game/ShootingRange/Audio/手雷爆炸.手雷爆炸" _returnvalue "0, 0, 0" 1.0 1.0 0.0 0 0 0)
  (Effects|SpawnEmitteratLocation "/Game/FXVarietyPack/P_ky_explosion.P_ky_explosion" _returnvalue)
  (bind (_outhits _returnvalue_2) (Collision|MultiSphereTraceForObjects _returnvalue _returnvalue 3.5e+02 (Utilities|Array|MakeArray "ObjectTypeQuery4") false 0 "ForDuration"))
  (Development|SetHiddeninGame (Variables|Default|GetStaticMesh) true false)
  (Actor|SetLifeSpan 2.0)
  (if _returnvalue_2
    (for _array_element _outhits
      (Game|Damage|ApplyDamage (.HitActor (Collision|BreakHitResult _array_element)) (Variables|Default|GetDamege) 0 0)
      (if (Physics|IsSimulatingPhysics (.HitComponent (Collision|BreakHitResult _array_element)) "None")
        (Physics|AddImpulseatLocation (.HitComponent (Collision|BreakHitResult _array_element)) (* (Math|Vector|GetUnitDirection(Vector) (Transformation|GetWorldLocation (Variables|Default|GetStaticMesh)) (Transformation|GetWorldLocation (.HitComponent (Collision|BreakHitResult _array_element)))) (Variables|Default|GetImpulse)) (.Location (Collision|BreakHitResult _array_element)) "None")))))

(event EventBeginPlay)

(event Collision|EventActorBeginOverlap
  (params (OtherActor :type Actor%20Object%20Reference)))

(event EventTick
  (params (DeltaSeconds :type Float%20%28single-precision%29)))

(fn ConstructionScript)