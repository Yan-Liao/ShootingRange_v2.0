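; Base weapon for the shooting range, handling pickup, firing, reloading, fire-mode cycling, a toggleable light and UI info.
; Fire modes are single, counted burst (Semi-Auto), full-auto and shotgun (My Gun), with bursts and full-auto looping on montage completion.
; Fire montage notifies spawn BP_ProjectileBase at the muzzle, aimed at the owner's LookAtPoint, or muzzle-forward beyond 90° yaw.
; Shotgun pellets add random world-XY circle offsets scaled by target distance.
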(event Custom|ReloadWeapon
  (Variables|Default|SetRoundsInChamber (Variables|Default|GetMagSize))
  (Animation|Montage|PlayMontage (Variables|Default|GetSkeletalMesh) (Variables|Default|GetReloadMontageWeapon)
    (:then
      (Audio|PlaySound2D (Variables|Default|GetReloadSound) 1.0 1.0 0.0 0 0))))

(event Custom|Fire
  (bind _owning_character (Variables|Default|GetOwning%20Character))
  (bind _skeletalmesh (Variables|Default|GetSkeletalMesh))
  (bind _owning_character_2 (Variables|Default|GetOwning%20Character))
  (bind _skeletalmesh_2 (Variables|Default|GetSkeletalMesh))
  (bind _rbm (Variables|Default|GetRBM))
  (bind _rbm_2 (Variables|Default|GetRBM))
  (bind _rbm_3 (Variables|Default|GetRBM))
  (bind _returnvalue (Transformation|GetSocketRotation _skeletalmesh "Muzzle"))
  (bind _returnvalue_2 (/ _rbm 2e+02))
  (bind _returnvalue_3 (/ _rbm_2 2e+02))
  (bind _returnvalue_4 (/ _rbm_3 2e+02))
  (bind _returnvalue_5 (Transformation|GetSocketLocation _skeletalmesh_2 "Muzzle"))
  (bind _lookatpoint (Variables|/Game/ShootingRange/Blueprints/Character/BP_MyCharacter.BP_MyCharacter_C|GetLookAtPoint _owning_character_2))
  (bind _yaw (Variables|/Game/ShootingRange/Blueprints/Character/BP_MyCharacter.BP_MyCharacter_C|GetYaw _owning_character))
  (bind _returnvalue_6 (Math|Float|Absolute(Float) _yaw))
  (bind _returnvalue_7 (Math|Vector|GetForwardVector _returnvalue))
  (bind _returnvalue_8 (- _lookatpoint _returnvalue_5))
  (bind _returnvalue_9 (>= _returnvalue_6 9e+01))
  (bind _returnvalue_10 (Math|Vector|SelectVector _returnvalue_7 _returnvalue_8 _returnvalue_9))
  (bind (_x _y _z) (Math|Vector|BreakVector _returnvalue_10))
  (switch Utilities|FlowControl|Switch|SwitchonEFireMode (Variables|Default|GetFireMode)
    (:NewEnumerator0
      (Utilities|FlowControl|DoOnce false :!label _label
        (:Completed
          (Animation|Montage|PlayMontage (Variables|/Script/Engine.Character|GetMesh (Variables|Default|GetOwning%20Character)) "/Game/ShootingRange/Assets/Character/Animations/AM_2HW_ADS_Fire.AM_2HW_ADS_Fire" _returnvalue_4
            (:then
              (Animation|Montage|PlayMontage (Variables|Default|GetSkeletalMesh) (Variables|Default|GetFireMontageWeapon) _returnvalue_4))
            (:OnCompleted
              (goto _label Reset))
            (:OnNotifyBegin
              (Audio|PlaySound2D (Variables|Default|GetFireSound) 1.0 1.0 0.0 0 0)
              (bind _returnvalue_11 (Game|SpawnActorfromClass "/Game/ShootingRange/Blueprints/Weapons/BP_ProjectileBase.BP_ProjectileBase_C" (Transformation|GetSocketTransform (Variables|Default|GetSkeletalMesh) "Muzzle" "RTS_World") "AlwaysSpawn" 0 0 :!label _label_2))
              (Variables|/Script/Engine.MovementComponent|SetVelocity (Variables|/Game/ShootingRange/Blueprints/Weapons/BP_ProjectileBase.BP_ProjectileBase_C|GetProjectileMovement _returnvalue_11) (* (Math|Vector|Normalize (Math|Vector|SelectVector (Math|Vector|GetForwardVector (Transformation|GetSocketRotation (Variables|Default|GetSkeletalMesh) "Muzzle")) (- (Variables|/Game/ShootingRange/Blueprints/Character/BP_MyCharacter.BP_MyCharacter_C|GetLookAtPoint (Variables|Default|GetOwning%20Character)) (Transformation|GetSocketLocation (Variables|Default|GetSkeletalMesh) "Muzzle")) (>= (Math|Float|Absolute(Float) (Variables|/Game/ShootingRange/Blueprints/Character/BP_MyCharacter.BP_MyCharacter_C|GetYaw (Variables|Default|GetOwning%20Character))) 9e+01))) (Variables|Default|GetMuzzleVelocity)))
              (Math|Integer|DecrementInt (Variables|Default|GetRoundsInChamber)))))))
    (:NewEnumerator2
      (Animation|Montage|PlayMontage (Variables|/Script/Engine.Character|GetMesh (Variables|Default|GetOwning%20Character)) "/Game/ShootingRange/Assets/Character/Animations/AM_2HW_ADS_Fire.AM_2HW_ADS_Fire" _returnvalue_3
        (:then
          (Animation|Montage|PlayMontage (Variables|Default|GetSkeletalMesh) (Variables|Default|GetFireMontageWeapon) _returnvalue_3))
        (:OnCompleted
          (Math|Integer|IncrementInt (Variables|Default|GetFireNum)
            (:%20%20
              (CallFunction|ShouldRepeatCheckSemiAuto))))
        (:OnNotifyBegin
          (Audio|PlaySound2D (Variables|Default|GetFireSound) 1.0 1.0 0.0 0 0)
          (goto _label_2))))
    (:NewEnumerator3
      (Animation|Montage|PlayMontage (Variables|/Script/Engine.Character|GetMesh (Variables|Default|GetOwning%20Character)) "/Game/ShootingRange/Assets/Character/Animations/AM_2HW_ADS_Fire.AM_2HW_ADS_Fire" _returnvalue_2
        (:then
          (Animation|Montage|PlayMontage (Variables|Default|GetSkeletalMesh) (Variables|Default|GetFireMontageWeapon) _returnvalue_2))
        (:OnCompleted
          (CallFunction|ShouldRepeatCheckFullAuto))
        (:OnNotifyBegin
          (Audio|PlaySound2D (Variables|Default|GetFireSound) 1.0 1.0 0.0 0 0)
          (goto _label_2))))
    (:NewEnumerator4
      (Utilities|FlowControl|DoOnce false :!label _label_3
        (:Completed
          (Math|Integer|DecrementInt (Variables|Default|GetRoundsInChamber)
            (:%20%20
              (Animation|Montage|PlayMontage (Variables|/Script/Engine.Character|GetMesh (Variables|Default|GetOwning%20Character)) "/Game/ShootingRange/Assets/Character/Animations/AM_2HW_ADS_Fire.AM_2HW_ADS_Fire" (/ (Variables|Default|GetRBM) 2e+02)
                (:OnNotifyBegin
                  (Audio|PlaySound2D (Variables|Default|GetFireSound) 1.0 1.0 0.0 0 0)
                  (for _index (range 1 (Variables|Default|GetShotGunBurstNum))
                    (Variables|Default|SetShotGunDistance (Math|Vector|VectorLength _returnvalue_10))
                    (bind _point (CallFunction|RandPointinCircle (* (Math|Trig|Tan(Degrees) (Variables|Default|GetShotGunBulletAngle)) (Variables|Default|GetShotGunDistance))))
                    (Variables|Default|SetShotGunRandomCircle _point)
                    (bind _returnvalue_12 (Game|SpawnActorfromClass "/Game/ShootingRange/Blueprints/Weapons/BP_ProjectileBase.BP_ProjectileBase_C" (Transformation|GetSocketTransform (Variables|Default|GetSkeletalMesh) "Muzzle" "RTS_World") "AlwaysSpawn" 0 0))
                    (Variables|/Script/Engine.MovementComponent|SetVelocity (Variables|/Game/ShootingRange/Blueprints/Weapons/BP_ProjectileBase.BP_ProjectileBase_C|GetProjectileMovement _returnvalue_12) (* (Math|Vector|Normalize (Math|Vector|MakeVector (+ (.x (Variables|Default|GetShotGunRandomCircle)) _x) (+ (.y (Variables|Default|GetShotGunRandomCircle)) _y) _z)) (Variables|Default|GetMuzzleVelocity))))
                  (Utilities|FlowControl|Delay 0.4)
                  (goto _label_3 Reset))))))))))

(event Custom|FireRelease
  (Variables|Default|SetIsFiring false))

(event Custom|RepeatFire
  (bind _owning_character (Variables|Default|GetOwning%20Character))
  (bind _skeletalmesh (Variables|Default|GetSkeletalMesh))
  (bind _owning_character_2 (Variables|Default|GetOwning%20Character))
  (bind _skeletalmesh_2 (Variables|Default|GetSkeletalMesh))
  (bind _rbm (Variables|Default|GetRBM))
  (bind _rbm_2 (Variables|Default|GetRBM))
  (bind _rbm_3 (Variables|Default|GetRBM))
  (bind _returnvalue (Transformation|GetSocketRotation _skeletalmesh "Muzzle"))
  (bind _returnvalue_2 (/ _rbm 2e+02))
  (bind _returnvalue_3 (/ _rbm_2 2e+02))
  (bind _returnvalue_4 (/ _rbm_3 2e+02))
  (bind _returnvalue_5 (Transformation|GetSocketLocation _skeletalmesh_2 "Muzzle"))
  (bind _lookatpoint (Variables|/Game/ShootingRange/Blueprints/Character/BP_MyCharacter.BP_MyCharacter_C|GetLookAtPoint _owning_character_2))
  (bind _yaw (Variables|/Game/ShootingRange/Blueprints/Character/BP_MyCharacter.BP_MyCharacter_C|GetYaw _owning_character))
  (bind _returnvalue_6 (Math|Float|Absolute(Float) _yaw))
  (bind _returnvalue_7 (Math|Vector|GetForwardVector _returnvalue))
  (bind _returnvalue_8 (- _lookatpoint _returnvalue_5))
  (bind _returnvalue_9 (>= _returnvalue_6 9e+01))
  (bind _returnvalue_10 (Math|Vector|SelectVector _returnvalue_7 _returnvalue_8 _returnvalue_9))
  (bind (_x _y _z) (Math|Vector|BreakVector _returnvalue_10))
  (switch Utilities|FlowControl|Switch|SwitchonEFireMode (Variables|Default|GetFireMode)
    (:NewEnumerator0
      (Utilities|FlowControl|DoOnce false :!label _label
        (:Completed
          (Animation|Montage|PlayMontage (Variables|/Script/Engine.Character|GetMesh (Variables|Default|GetOwning%20Character)) "/Game/ShootingRange/Assets/Character/Animations/AM_2HW_ADS_Fire.AM_2HW_ADS_Fire" _returnvalue_4
            (:then
              (Animation|Montage|PlayMontage (Variables|Default|GetSkeletalMesh) (Variables|Default|GetFireMontageWeapon) _returnvalue_4))
            (:OnCompleted
              (goto _label Reset))
            (:OnNotifyBegin
              (Audio|PlaySound2D (Variables|Default|GetFireSound) 1.0 1.0 0.0 0 0)
              (bind _returnvalue_11 (Game|SpawnActorfromClass "/Game/ShootingRange/Blueprints/Weapons/BP_ProjectileBase.BP_ProjectileBase_C" (Transformation|GetSocketTransform (Variables|Default|GetSkeletalMesh) "Muzzle" "RTS_World") "AlwaysSpawn" 0 0 :!label _label_2))
              (Variables|/Script/Engine.MovementComponent|SetVelocity (Variables|/Game/ShootingRange/Blueprints/Weapons/BP_ProjectileBase.BP_ProjectileBase_C|GetProjectileMovement _returnvalue_11) (* (Math|Vector|Normalize (Math|Vector|SelectVector (Math|Vector|GetForwardVector (Transformation|GetSocketRotation (Variables|Default|GetSkeletalMesh) "Muzzle")) (- (Variables|/Game/ShootingRange/Blueprints/Character/BP_MyCharacter.BP_MyCharacter_C|GetLookAtPoint (Variables|Default|GetOwning%20Character)) (Transformation|GetSocketLocation (Variables|Default|GetSkeletalMesh) "Muzzle")) (>= (Math|Float|Absolute(Float) (Variables|/Game/ShootingRange/Blueprints/Character/BP_MyCharacter.BP_MyCharacter_C|GetYaw (Variables|Default|GetOwning%20Character))) 9e+01))) (Variables|Default|GetMuzzleVelocity)))
              (Math|Integer|DecrementInt (Variables|Default|GetRoundsInChamber)))))))
    (:NewEnumerator2
      (Animation|Montage|PlayMontage (Variables|/Script/Engine.Character|GetMesh (Variables|Default|GetOwning%20Character)) "/Game/ShootingRange/Assets/Character/Animations/AM_2HW_ADS_Fire.AM_2HW_ADS_Fire" _returnvalue_3
        (:then
          (Animation|Montage|PlayMontage (Variables|Default|GetSkeletalMesh) (Variables|Default|GetFireMontageWeapon) _returnvalue_3))
        (:OnCompleted
          (Math|Integer|IncrementInt (Variables|Default|GetFireNum)
            (:%20%20
              (CallFunction|ShouldRepeatCheckSemiAuto))))
        (:OnNotifyBegin
          (Audio|PlaySound2D (Variables|Default|GetFireSound) 1.0 1.0 0.0 0 0)
          (goto _label_2))))
    (:NewEnumerator3
      (Animation|Montage|PlayMontage (Variables|/Script/Engine.Character|GetMesh (Variables|Default|GetOwning%20Character)) "/Game/ShootingRange/Assets/Character/Animations/AM_2HW_ADS_Fire.AM_2HW_ADS_Fire" _returnvalue_2
        (:then
          (Animation|Montage|PlayMontage (Variables|Default|GetSkeletalMesh) (Variables|Default|GetFireMontageWeapon) _returnvalue_2))
        (:OnCompleted
          (CallFunction|ShouldRepeatCheckFullAuto))
        (:OnNotifyBegin
          (Audio|PlaySound2D (Variables|Default|GetFireSound) 1.0 1.0 0.0 0 0)
          (goto _label_2))))
    (:NewEnumerator4
      (Utilities|FlowControl|DoOnce false :!label _label_3
        (:Completed
          (Math|Integer|DecrementInt (Variables|Default|GetRoundsInChamber)
            (:%20%20
              (Animation|Montage|PlayMontage (Variables|/Script/Engine.Character|GetMesh (Variables|Default|GetOwning%20Character)) "/Game/ShootingRange/Assets/Character/Animations/AM_2HW_ADS_Fire.AM_2HW_ADS_Fire" (/ (Variables|Default|GetRBM) 2e+02)
                (:OnNotifyBegin
                  (Audio|PlaySound2D (Variables|Default|GetFireSound) 1.0 1.0 0.0 0 0)
                  (for _index (range 1 (Variables|Default|GetShotGunBurstNum))
                    (Variables|Default|SetShotGunDistance (Math|Vector|VectorLength _returnvalue_10))
                    (bind _point (CallFunction|RandPointinCircle (* (Math|Trig|Tan(Degrees) (Variables|Default|GetShotGunBulletAngle)) (Variables|Default|GetShotGunDistance))))
                    (Variables|Default|SetShotGunRandomCircle _point)
                    (bind _returnvalue_12 (Game|SpawnActorfromClass "/Game/ShootingRange/Blueprints/Weapons/BP_ProjectileBase.BP_ProjectileBase_C" (Transformation|GetSocketTransform (Variables|Default|GetSkeletalMesh) "Muzzle" "RTS_World") "AlwaysSpawn" 0 0))
                    (Variables|/Script/Engine.MovementComponent|SetVelocity (Variables|/Game/ShootingRange/Blueprints/Weapons/BP_ProjectileBase.BP_ProjectileBase_C|GetProjectileMovement _returnvalue_12) (* (Math|Vector|Normalize (Math|Vector|MakeVector (+ (.x (Variables|Default|GetShotGunRandomCircle)) _x) (+ (.y (Variables|Default|GetShotGunRandomCircle)) _y) _z)) (Variables|Default|GetMuzzleVelocity))))
                  (Utilities|FlowControl|Delay 0.4)
                  (goto _label_3 Reset))))))))))

(event Custom|ToggleFireModeWeapon
  (if (> (Utilities|Array|Length (Variables|Default|GetAvailableFireMode)) 1)
    (bind _nextitem (Utilities|GetArrayNextItem (Variables|Default|GetAvailableFireMode) (Variables|Default|GetFireMode))
      (:Out
        (Variables|Default|SetFireMode _nextitem)
        (Audio|PlaySound2D "/Game/ShootingRange/Audio/换切开火.换切开火" 1.0 1.0 0.0 0 0)))))

(event Custom|OpenLight
  (Rendering|Components|Light|SetIntensity (Variables|Default|GetSpotLight) (Variables|Default|GetLightIntensity)))

(event Custom|CloseLight
  (Rendering|Components|Light|SetIntensity (Variables|Default|GetSpotLight) 0.0))

(event EventFireWeapon
  (if (> (Variables|Default|GetRoundsInChamber) 0)
    (Variables|Default|SetIsFiring true)
    (CallFunction|Fire)
    (else
      (Audio|PlaySound2D "/Game/ShootingRange/Audio/空膛.空膛" 1.0 1.0 0.0 0 0))))

(event EventGetWeapon
  (params (OwningCharacter :type BP%20My%20Character%20Object%20Reference))
  (Variables|Default|SetOwning%20Character OwningCharacter)
  (Physics|SetSimulatePhysics (Variables|Default|GetSkeletalMesh) false)
  (Components|DestroyComponent (Variables|Default|GetCapsule))
  (Variables|Default|SetAimBaselineOffset (- (Class|KismetAnimationLibrary|DistanceBetweenTwoSocketsandMapRange (Variables|Default|GetSkeletalMesh) "Root" "RTS_World" "Sight" "RTS_World" false 0.0 0.0 0.0 0.0) 13.53)))

(fn ConstructionScript)

(fn ShouldRepeatCheckSemiAuto
  (if (and (> (Variables|Default|GetRoundsInChamber) 0) (< (Variables|Default|GetFireNum) (Variables|Default|GetSimeFireNum)))
    (CallFunction|RepeatFire)
    (else
      (if (< (Variables|Default|GetFireNum) (Variables|Default|GetSimeFireNum))
        (Audio|PlaySound2D "/Game/ShootingRange/Audio/空膛.空膛" 1.0 1.0 0.0 0 0))
      (Variables|Default|SetFireNum 0))))

(fn RandPointinCircle
  (params (Radius :type Float%20%28single-precision%29))
  (LocalVariables|SetDistanceFromCenter (Math|Random|RandomFloatinRange 0.0 Radius))
  (LocalVariables|SetAngle (Math|Random|RandomFloatinRange 0.0 3.6e+02))
  (return (Math|Vector2D|MakeVector2D (* (LocalVariables|GetDistanceFromCenter) (Math|Trig|Cos(Degrees) (LocalVariables|GetAngle))) (* (Math|Trig|Sin(Degrees) (LocalVariables|GetAngle)) (LocalVariables|GetDistanceFromCenter)))))

(fn ShouldRepeatCheckFullAuto
  (bind _isfiring (Variables|Default|GetIsFiring))
  (if (and _isfiring (> (Variables|Default|GetRoundsInChamber) 0))
    (CallFunction|RepeatFire)
    (elif _isfiring
      (Audio|PlaySound2D "/Game/ShootingRange/Audio/空膛.空膛" 1.0 1.0 0.0 0 0))))

(fn GetWeaponPanelInfo
  (return self (Variables|Default|GetWeaponType)))

(fn SendValue
  (return (Utilities|Struct|MakeSWeaponSendValue (Variables|Default|GetWeaponName) (Variables|Default|GetFireMode) (Variables|Default|GetRoundsInChamber) (Variables|Default|GetMagSize))))