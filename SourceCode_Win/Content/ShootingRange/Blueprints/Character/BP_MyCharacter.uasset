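; Player character for a shooting game, handling weapons, grenades, stamina sprinting, health with mission failure on death, and door and hostage interaction.
; A head-to-aim sphere trace drives interaction and pickup into holster slots, with montages and socket attachment for switching.
; Tick computes aim, movement and left-hand IK grip values, exposed through SendValue.
; Holding grenade input redraws a predicted spline-mesh arc and landing decal, and release launches it.
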(event Custom|loss_stamina
  ;[1 1 1] shift奔跑
  (bind _output_get (Variables|Default|Setstamina (Math|Float|Max(Float) (- (Variables|Default|Getstamina) (Variables|Default|Getstamina_cost)) 0.0)))
  (Math|Float|CompareFloat _output_get 0.0
    (:==
      _)
    (:<
      _))
  (Variables|/Script/Engine.CharacterMovementComponent|SetMaxWalkSpeed (Variables|Character|GetCharacterMovement) (Variables|Default|GetWalkSpeed))
  (Utilities|Time|ClearTimerbyFunctionName 0 "loss_stamina")
  (Utilities|Time|SetTimerbyFunctionName 0 "recover_stamina" 0.1 true))

(event Custom|recover_stamina
  ;[1 1 1] shift奔跑
  (bind _output_get (Variables|Default|Setstamina (Math|Float|Min(Float) (+ (Variables|Default|Getstamina) (Variables|Default|Getstamina_recover)) (Variables|Default|GetMaxStamina))))
  (Math|Float|CompareFloat _output_get (Variables|Default|GetMaxStamina)
    (:>
      _)
    (:==
      _))
  (Utilities|Time|ClearTimerbyFunctionName 0 "recover_stamina"))

(event Custom|HolsterWeapon
  ;[1 1 1] EquipWeapon
  (CallFunction|CloseWeaponLight)
  (Variables|Default|SetIsCombate false)
  (Animation|Montage|PlayMontage (Variables|Character|GetMesh) (Utilities|Array|Get(acopy) (Variables|Default|GetHolsterMontage) (Variables|Default|GetCurrentWeaponSlotsIndex))))

(event Custom|CallWeaponSlot
  (bind _weaponslotsindex (Variables|Default|GetWeaponSlotsIndex))
  ;[1 1 1] EquipWeapon
  (if (Math|Boolean|ANDBoolean (not (Variables|Default|GetIsChangingWeapon)) (!= (.weaponbase (Utilities|Array|Get(acopy) (Variables|Default|GetWeaponSlots) (Variables|Default|GetWeaponSlotsIndex))) 0) (CallFunction|MontageIsNotRunning))
    (Variables|Default|SetIsChangingWeapon true)
    (if (Variables|Default|GetIsCombate)
      (if (!= (Variables|Default|GetCurrentWeaponSlotsIndex) _weaponslotsindex)
        (CallFunction|CloseWeaponLight)
        (Variables|Default|SetIsCombate false)
        (Animation|Montage|PlayMontage (Variables|Character|GetMesh) (Utilities|Array|Get(acopy) (Variables|Default|GetHolsterMontage) (Variables|Default|GetCurrentWeaponSlotsIndex))
          (:OnBlendOut
            (Variables|Default|SetCurrentWeaponSlotsIndex (Variables|Default|GetWeaponSlotsIndex))
            (CallFunction|EquipWeapon)
            (Variables|Default|SetIsChangingWeapon false)))
        (else
          (CallFunction|HolsterWeapon)
          (Variables|Default|SetIsChangingWeapon false)))
      (else
        (Variables|Default|SetCurrentWeaponSlotsIndex _weaponslotsindex)
        (CallFunction|EquipWeapon)
        (Variables|Default|SetIsChangingWeapon false)))))

(event Custom|HolsterWeaponBR
  (bind (_weapon_base _weapon_type _holster) (CallFunction|GetCurrentWeaponSlot))
  ;[1 1 1] EquipWeapon
  (Transformation|AttachComponentToComponent _weapon_base (Variables|Character|GetMesh) _holster "SnapToTarget" "SnapToTarget" "SnapToTarget" true))

(event Custom|EquipWeaponBR
  ;[1 1 1] EquipWeapon
  (Transformation|AttachComponentToComponent (.Weapon%20Base (CallFunction|GetCurrentWeaponSlot)) (Variables|Character|GetMesh) "HandRSocket" "SnapToTarget" "SnapToTarget" "SnapToTarget" true)
  (Variables|Default|SetAim%20Baseline%20Offset (Variables|/Game/ShootingRange/Blueprints/Weapons/BP_WeaponBase.BP_WeaponBase_C|GetAimBaselineOffset (.Weapon%20Base (CallFunction|GetCurrentWeaponSlot)))))

(event Custom|DebugFlow
  (params (Debug :type Boolean))
  ;[1 1 1] DebugFlow
  (if Debug
    (Development|PrintString (Utilities|String|Append "Yaw" (Utilities|String|ToString(Float) (Variables|Default|GetYaw))) true true "(R=0.000000,G=0.660000,B=1.000000,A=1.000000)" 0.0)
    (Development|PrintString (Utilities|String|Append "Pitch" (Utilities|String|ToString(Float) (Variables|Default|GetPitch))) true true "(R=0.000000,G=0.660000,B=1.000000,A=1.000000)" 0.0)))

(event Custom|PickUpWeapon
  (bind (_weapon_base _weapon_type _holster) (CallFunction|GetWeaponSlot))
  (bind _weaponpanelinfo (Variables|Default|GetWeaponPanelInfo))
  ;[1 1 1] PickUpWeapon/OpenDoor/SaveHostage
  (if (Variables|Default|GetScannerWeapon)
    (bind (_array_element _array_index) (Utilities|Array|ForEachLoopwithBreak (Variables|Default|GetWeaponSlots) :!label _label)
      (:LoopBody
        (if (and (== (.WeaponBase (Utilities|Struct|BreakSWeaponSlot _array_element)) 0) (Utilities|Enum|Equal(Enum) (.WeaponType (Utilities|Struct|BreakSWeaponSlot _array_element)) (.weapontype (Variables|Default|GetWeaponPanelInfo))))
          (Variables|Default|SetWeaponSlotsIndex _array_index)
          (Class|BPIWeaponBase|GetWeapon(Message) (.weaponbase _weaponpanelinfo) self)
          (Utilities|Array|SetArrayElem (Variables|Default|GetWeaponSlots) (Variables|Default|GetWeaponSlotsIndex) (Utilities|Struct|MakeSWeaponSlot (.weaponbase _weaponpanelinfo) _weapon_type _holster))
          (Transformation|AttachComponentToComponent (.weaponbase _weaponpanelinfo) (Variables|Character|GetMesh) _holster "SnapToTarget" "SnapToTarget" "SnapToTarget" true)
          (Utilities|Array|AddUnique (Variables|Default|GetWeaponIndexList) (Variables|Default|GetWeaponSlotsIndex))
          (goto _label Break))))))

(event Custom|GrabWeaponBLTemp
  ;[1 1 1] EquipWeapon
  (Transformation|AttachComponentToComponent (.Weapon%20Base (CallFunction|GetCurrentWeaponSlot)) (Variables|Character|GetMesh) "HandLSocket" "KeepRelative" "KeepRelative" "KeepRelative" true))

(event Custom|ThrowedGrena
  (params (LaunchVelocity :type Vector))
  (bind _mesh (Variables|Character|GetMesh))
  (bind _returnvalue (Transformation|GetSocketTransform _mesh "HandRGrenadeSocket" "RTS_World"))
  ;[1 1 1] Throw Grenade
  (bind _returnvalue_2 (Game|SpawnActorfromClass "/Game/ShootingRange/Blueprints/Weapons/BP_Grenade.BP_Grenade_C" (Math|Transform|MakeTransform (.location _returnvalue) (.rotation _returnvalue) "3.000000,3.000000,3.000000") "AlwaysSpawn" 0 0))
  (Variables|/Script/Engine.MovementComponent|SetVelocity (Variables|/Game/ShootingRange/Blueprints/Weapons/BP_Grenade.BP_Grenade_C|GetProjectileMovement _returnvalue_2) LaunchVelocity)
  (Default|ThrowedGrenade _returnvalue_2))

(event Custom|EquipWeapon
  ;[1 1 1] EquipWeapon
  (Variables|Default|SetIsCombate true)
  (Animation|Montage|PlayMontage (Variables|Character|GetMesh) (Utilities|Array|Get(acopy) (Variables|Default|GetEquipMontage) (Variables|Default|GetCurrentWeaponSlotsIndex))))

(event Game|Damage|EventAnyDamage
  (params (Damage :type Float%20%28single-precision%29) (DamageType :type Damage%20Type%20Object%20Reference) (InstigatedBy :type Controller%20Object%20Reference) (DamageCauser :type Actor%20Object%20Reference))
  ;[1 1 1] GotDamage
  (bind _output_get (Variables|Default|Sethp (Math|Float|Max(Float) (- (Variables|Default|Gethp) Damage) 0.0)))
  (Math|Float|CompareFloat _output_get 1.0
    (:==
      _)
    (:<
      _))
  (Utilities|FlowControl|DoOnce false
    (:Completed
      (Class|Pawn|DetachfromControllerPendingDestroy)
      (Animation|Montage|PlayMontage (Variables|Character|GetMesh) "/Game/ShootingRange/Assets/Character/Animations/AM_MOB1_Stand_Relaxed_Death_B_IPC.AM_MOB1_Stand_Relaxed_Death_B_IPC"
        (:OnNotifyBegin
          (Class|BPIMyGameState|MissionFailed(Message) (Game|GetGameState) "NewEnumerator0"))))))

(event EventBeginPlay
  (Variables|Default|SetHp (Variables|Default|GetMaxHp))
  (Variables|Default|SetStamina (Variables|Default|GetMaxStamina)))

(event EventTick
  (params (DeltaSeconds :type Float%20%28single-precision%29))
  (bind _returnvalue (Pawn|GetBaseAimRotation))
  (bind _returnvalue_2 (Transformation|GetActorRotation))
  (bind _returnvalue_3 (Transformation|GetVelocity))
  (bind _returnvalue_4 (Math|Rotator|Delta(Rotator) _returnvalue _returnvalue_2))
  ;[1 1 1] Tick
  (Variables|Default|SetIsInAir (AI|Components|NavMovement|IsFalling (Variables|Character|GetCharacterMovement)))
  (Variables|Default|SetSpeed (Math|Vector|VectorLength _returnvalue_3))
  (Variables|Default|SetDirction (Class|AnimInstance|CalculateDirection (Components|SkeletalMesh|GetAnimInstance (Variables|Character|GetMesh)) _returnvalue_3 (Transformation|GetActorRotation)))
  (Variables|Default|SetPitch (.pitch _returnvalue_4))
  (Variables|Default|SetYaw (.yaw _returnvalue_4))
  (Variables|Default|SetLookAtPoint (CallFunction|ActorLookatPoint))
  (CallFunction|ToggleHandLIK)
  (CallFunction|CaculateLHandOfset)
  (CallFunction|GetCurrentWeaponValue))

(event Input|ActionEvents|InputActionToggleFireMode
  (params (Key :type Key%20Structure :default "None"))
  (bind _weapon_base (CallFunction|GetCurrentWeaponSlot))
  ;[1 1 1] Fire/ToggleFireMode
  (:Pressed
    (if (Math|Boolean|ANDBoolean (Variables|Default|GetIsCombate) (not (Variables|Default|GetIsReloading)) (not (Variables|/Game/ShootingRange/Blueprints/Weapons/BP_WeaponBase.BP_WeaponBase_C|GetIsFiring _weapon_base)))
      (Default|ToggleFireModeWeapon _weapon_base))))

(event Input|ActionEvents|InputActionOpenLight
  (params (Key :type Key%20Structure :default "None"))
  (:Pressed
    (if (Variables|Default|GetIsCombate)
      (if (Variables|Default|GetIsLightOpen)
        (CallFunction|CloseWeaponLight)
        (else
          (CallFunction|OpenWeaponLight))))))

(event Input|ActionEvents|InputActionPreWeapon
  (params (Key :type Key%20Structure :default "None"))
  ;[1 1 1] EquipWeapon
  (:Pressed
    (if (Math|Boolean|ANDBoolean (!= (Utilities|Array|Length (Variables|Default|GetWeaponIndexList)) 0) (CallFunction|MontageIsNotRunning) (not (Variables|Default|GetIsChangingWeapon)))
      (Variables|Default|SetIsChangingWeapon true)
      (if (!= (.Weapon%20Base (CallFunction|GetCurrentWeaponSlot)) 0)
        (if (not (Variables|Default|GetIsCombate))
          (CallFunction|EquipWeapon)
          (Variables|Default|SetIsChangingWeapon false)
          (else
            (bind _nextweaponindex (Utilities|GetPreWeapon (Variables|Default|GetWeaponIndexList) (Variables|Default|GetCurrentWeaponSlotsIndex))
              (:Out
                (if (!= _nextweaponindex (Variables|Default|GetCurrentWeaponSlotsIndex))
                  (CallFunction|CloseWeaponLight)
                  (Variables|Default|SetIsCombate false)
                  (Animation|Montage|PlayMontage (Variables|Character|GetMesh) (Utilities|Array|Get(acopy) (Variables|Default|GetHolsterMontage) (Variables|Default|GetCurrentWeaponSlotsIndex))
                    (:OnBlendOut
                      (Variables|Default|SetCurrentWeaponSlotsIndex _nextweaponindex)
                      (CallFunction|EquipWeapon)
                      (Variables|Default|SetIsChangingWeapon false)))
                  (else
                    (Variables|Default|SetIsChangingWeapon false)))))))
        (else
          (bind _nextweaponindex_2 (Utilities|GetPreWeapon (Variables|Default|GetWeaponIndexList) (Variables|Default|GetCurrentWeaponSlotsIndex))
            (:Out
              (Variables|Default|SetCurrentWeaponSlotsIndex _nextweaponindex_2)
              (CallFunction|EquipWeapon)
              (Variables|Default|SetIsChangingWeapon false))))))))

(event Input|ActionEvents|InputActionNextWeapon
  (params (Key :type Key%20Structure :default "None"))
  ;[1 1 1] EquipWeapon
  (:Pressed
    (if (Math|Boolean|ANDBoolean (!= (Utilities|Array|Length (Variables|Default|GetWeaponIndexList)) 0) (CallFunction|MontageIsNotRunning) (not (Variables|Default|GetIsChangingWeapon)))
      (if (!= (.Weapon%20Base (CallFunction|GetCurrentWeaponSlot)) 0)
        (if (not (Variables|Default|GetIsCombate))
          (CallFunction|EquipWeapon)
          (Variables|Default|SetIsChangingWeapon false)
          (else
            (bind _nextweaponindex (Utilities|GetNextWeapon (Variables|Default|GetWeaponIndexList) (Variables|Default|GetCurrentWeaponSlotsIndex))
              (:Out
                (if (!= _nextweaponindex (Variables|Default|GetCurrentWeaponSlotsIndex))
                  (CallFunction|CloseWeaponLight)
                  (Variables|Default|SetIsCombate false)
                  (Animation|Montage|PlayMontage (Variables|Character|GetMesh) (Utilities|Array|Get(acopy) (Variables|Default|GetHolsterMontage) (Variables|Default|GetCurrentWeaponSlotsIndex))
                    (:OnBlendOut
                      (Variables|Default|SetCurrentWeaponSlotsIndex _nextweaponindex)
                      (CallFunction|EquipWeapon)
                      (Variables|Default|SetIsChangingWeapon false)))
                  (else
                    (Variables|Default|SetIsChangingWeapon false)))))))
        (else
          (bind _nextweaponindex_2 (Utilities|GetNextWeapon (Variables|Default|GetWeaponIndexList) (Variables|Default|GetCurrentWeaponSlotsIndex))
            (:Out
              (Variables|Default|SetCurrentWeaponSlotsIndex _nextweaponindex_2)
              (CallFunction|EquipWeapon)
              (Variables|Default|SetIsChangingWeapon false))))))))

(event Input|ActionEvents|InputActionCallWeaponSlot1
  (params (Key :type Key%20Structure :default "None"))
  ;[1 1 1] EquipWeapon
  (:Pressed
    (Variables|Default|SetWeaponSlotsIndex 0)
    (CallFunction|CallWeaponSlot)))

(event Input|ActionEvents|InputActionCallWeaponSlot2
  (params (Key :type Key%20Structure :default "None"))
  ;[1 1 1] EquipWeapon
  (:Pressed
    (Variables|Default|SetWeaponSlotsIndex 1)
    (CallFunction|CallWeaponSlot)))

(event Input|ActionEvents|InputActionCallWeaponSlot3
  (params (Key :type Key%20Structure :default "None"))
  ;[1 1 1] EquipWeapon
  (:Pressed
    (Variables|Default|SetWeaponSlotsIndex 2)
    (CallFunction|CallWeaponSlot)))

(event Input|ActionEvents|InputActionHolsterWeapon
  (params (Key :type Key%20Structure :default "None"))
  ;[1 1 1] EquipWeapon
  (:Pressed
    (CallFunction|HolsterWeapon)))

(event Input|ActionEvents|InputActionRun
  (params (Key :type Key%20Structure :default "None"))
  (bind _charactermovement (Variables|Character|GetCharacterMovement))
  ;[1 1 1] shift奔跑
  (:Pressed
    (Variables|/Script/Engine.CharacterMovementComponent|SetMaxWalkSpeed _charactermovement (Variables|Default|GetRunSpeed))
    (Utilities|Time|ClearTimerbyFunctionName 0 "recover_stamina")
    (Utilities|Time|SetTimerbyFunctionName 0 "loss_stamina" 0.1 true))
  (:Released
    (Variables|/Script/Engine.CharacterMovementComponent|SetMaxWalkSpeed _charactermovement (Variables|Default|GetWalkSpeed))
    (Utilities|Time|ClearTimerbyFunctionName 0 "loss_stamina")
    (Utilities|Time|SetTimerbyFunctionName 0 "recover_stamina" 0.1 true)))

(event Input|ActionEvents|InputActionThrowGrenade
  (params (Key :type Key%20Structure :default "None"))
  (bind _mesh (Variables|Character|GetMesh))
  (bind _lookatpoint (Variables|Default|GetLookAtPoint))
  (bind _spline (Variables|Default|GetSpline))
  (bind _spline_2 (Variables|Default|GetSpline))
  (bind _returnvalue (Transformation|GetSocketLocation _mesh "HandRGrenadeSocket"))
  (bind _returnvalue_2 (- _lookatpoint _returnvalue))
  (bind _returnvalue_3 (Math|Vector|Normalize _returnvalue_2))
  (bind _returnvalue_4 (+ _returnvalue_3 "0, 0,0.300000"))
  (bind _returnvalue_5 (Math|Vector|Normalize _returnvalue_4))
  (bind _returnvalue_6 (* _returnvalue_5 1e+03))
  ;[1 1 1] Throw Grenade
  (:Pressed
    (Variables|Default|SetIsThrowing true)
    (|ClearSpline :!label _label
      (:execute
        (if (Variables|Default|GetIsThrowing)
          (bind (_outhit _outpathpositions _outlasttracedestination) (Class|GameplayStatics|BlueprintPredictProjectilePathbyTraceChannel _returnvalue _returnvalue_6 true 0.0 "ECC_WorldStatic" false (Utilities|Array|MakeArray self) "None" 3.0))
          (|DrawHitPoint _outlasttracedestination)
          (for (_array_element _array_index) _outpathpositions
            (Spline|AddSplinePointatIndex _spline_2 _array_element _array_index "Local" true))
          (for _index (range 0 (- (Spline|GetNumberOfSplinePoints _spline_2) 2))
            (bind _returnvalue_7 (AddComponent|AddSplineMeshComponent true (Math|Transform|MakeTransform "0, 0, 0")))
            (Utilities|Array|Add (Variables|Default|GetSplineMeshesArray) _returnvalue_7)
            (SplineMesh|SetStartandEnd _returnvalue_7 (Spline|GetLocationatSplinePoint _spline _index "Local") (Spline|GetTangentatSplinePoint _spline _index "Local") (Spline|GetLocationatSplinePoint _spline (+ _index 1) "Local") (Spline|GetTangentatSplinePoint _spline (+ _index 1) "Local") true :!class /Script/Engine.SplineMeshComponent))
          (Utilities|FlowControl|Delay (Utilities|Time|GetWorldDeltaSeconds))
          (goto _label)))))
  (:Released
    (Variables|Default|SetIsThrowing false)
    (Rendering|SetVisibility (Variables|Default|GetDecal) false false)
    (CallFunction|ThrowedGrena _returnvalue_6)))

(event Input|ActionEvents|InputActionReload
  (params (Key :type Key%20Structure :default "None"))
  ;[1 1 1] Reload
  (:Pressed
    (if (Variables|Default|GetIsCombate)
      (Variables|Default|SetIsReloading true)
      (Animation|Montage|PlayMontage (Variables|Character|GetMesh) (Variables|/Game/ShootingRange/Blueprints/Weapons/BP_WeaponBase.BP_WeaponBase_C|GetReloadMontageChar (.Weapon%20Base (CallFunction|GetCurrentWeaponSlot)))
        (:then
          (Default|ReloadWeapon (.Weapon%20Base (CallFunction|GetCurrentWeaponSlot))))
        (:OnCompleted
          (Variables|Default|SetIsReloading false :!label _label))
        (:OnBlendOut
          (goto _label))
        (:OnInterrupted
          (goto _label))))))

(event Input|ActionEvents|InputActionFire
  (params (Key :type Key%20Structure :default "None"))
  ;[1 1 1] Fire/ToggleFireMode
  (:Pressed
    (if (and (Variables|Default|GetIsCombate) (not (Variables|Default|GetIsReloading)))
      (Default|FireWeapon (.Weapon%20Base (CallFunction|GetCurrentWeaponSlot)))))
  (:Released
    (if (and (Variables|Default|GetIsCombate) (not (Variables|Default|GetIsReloading)))
      (Default|FireRelease (.Weapon%20Base (CallFunction|GetCurrentWeaponSlot))))))

(event Input|ActionEvents|InputActionPickUp
  (params (Key :type Key%20Structure :default "None"))
  (bind _mesh (Variables|Character|GetMesh))
  (bind _returnvalue (Transformation|GetSocketLocation _mesh "head"))
  ;[1 1 1] PickUpWeapon/OpenDoor/SaveHostage
  (:Pressed
    (bind (_outhit _returnvalue_2) (Collision|SphereTraceByChannel _returnvalue (+ _returnvalue (* (Math|Vector|Normalize (- (Variables|Default|GetLookAtPoint) _returnvalue)) 2e+02)) 3e+01 "TraceTypeQuery3" false 0 "None"))
    (if _returnvalue_2
      (Utilities|FlowControl|Sequence
        (:then_0
          (bind (_weaponbase _weapontype) (Class|BPIWeaponBase|GetWeaponPanelInfo(Message) (.HitActor (Collision|BreakHitResult _outhit))))
          (Variables|Default|SetWeaponPanelInfo (Utilities|Struct|MakeSWeaponPanelInfo _weaponbase _weapontype))
          (Variables|Default|SetScannerWeapon (Utilities|IsValid _weaponbase))
          (CallFunction|PickUpWeapon))
        (:then_1
          (bind _asbp_door (Utilities|Casting|CastToBP_Door (.HitActor (Collision|BreakHitResult _outhit))))
          (Default|OpenDoor _asbp_door))
        (:then_2
          (bind _asbp_hostage (Utilities|Casting|CastToBP_Hostage (.HitActor (Collision|BreakHitResult _outhit))))
          (Default|Saving _asbp_hostage))))))

(event Input|ActionEvents|InputActionADS
  (params (Key :type Key%20Structure :default "None"))
  ;[1 1 1] ADS
  (:Pressed
    (if (not (Variables|Default|GetIsALTWorking))
      (if (Variables|Default|GetIsCombate)
        (Variables|Default|SetIsADS true)
        (Variables|Default|SetbUseControllerRotationYaw true)
        (bind _新建轨道_0 (Timeline|时间轴_0 PlayFromStart)
          (:Update
            (Variables|/Script/Engine.CameraComponent|SetFieldOfView (Variables|Default|GetCamera) _新建轨道_0))))))
  (:Released
    (if (not (Variables|Default|GetIsALTWorking))
      (if (Variables|Default|GetIsCombate)
        (Variables|Default|SetIsADS false)
        (Variables|Default|SetbUseControllerRotationYaw false)
        (Timeline|时间轴_0 ReverseFromEnd)))))

(event Input|ActionEvents|InputActionADSForLong
  (params (Key :type Key%20Structure :default "None"))
  ;[1 1 1] ADS
  (:Pressed
    (Utilities|FlowControl|FlipFlop
      (:A
        (Variables|Default|SetIsALTWorking true)
        (if (Variables|Default|GetIsCombate)
          (Variables|Default|SetIsADS true)
          (Variables|Default|SetbUseControllerRotationYaw true)
          (bind _新建轨道_0 (Timeline|时间轴_0 PlayFromStart)
            (:Update
              (Variables|/Script/Engine.CameraComponent|SetFieldOfView (Variables|Default|GetCamera) _新建轨道_0)))))
      (:B
        (Variables|Default|SetIsALTWorking false)
        (if (Variables|Default|GetIsCombate)
          (Variables|Default|SetIsADS false)
          (Variables|Default|SetbUseControllerRotationYaw false)
          (Timeline|时间轴_0 ReverseFromEnd))))))

(fn ConstructionScript)

(fn CaculateLHandOfset
  (bind _weapon_base (CallFunction|GetCurrentWeaponSlot))
  (Utilities|IsValid _weapon_base
    (:Is%20Valid
      (Variables|Default|SetGripLOfset (.OutPosition (Class|SkinnedMeshComponent|TransformtoBoneSpace (Variables|Character|GetMesh) "hand_r" (.location (Transformation|GetSocketTransform (Variables|/Game/ShootingRange/Blueprints/Weapons/BP_WeaponBase.BP_WeaponBase_C|GetSkeletalMesh _weapon_base) "GripL" "RTS_World")) "0, 0, 0"))))))

(fn ToggleHandLIK
  (bind (_weapon_base _weapon_type) (CallFunction|GetCurrentWeaponSlot))
  (if (Math|Boolean|ANDBoolean (!= _weapon_base 0) (Utilities|Enum|Equal(Enum) _weapon_type "NewEnumerator0") (Variables|Default|GetIsCombate) (== (Animation|Curves|GetCurveValue (Components|SkeletalMesh|GetAnimInstance (Variables|Character|GetMesh)) "HandL IK Off") 0.0))
    (Variables|Default|SetUseLHandIK true)
    (else
      (Variables|Default|SetUseLHandIK false))))

(fn ActorLookatPoint
  (bind (_outhit _returnvalue) (Collision|LineTraceByChannel (Transformation|GetWorldLocation (Variables|Default|GetCamera)) (* (Math|Vector|GetForwardVector (Pawn|GetControlRotation :!class /Script/Engine.Pawn)) 1e+05) "TraceTypeQuery1" false 0 "ForOneFrame"))
  (return (Math|Vector|SelectVector (.Location (Collision|BreakHitResult _outhit)) (.TraceEnd (Collision|BreakHitResult _outhit)) _returnvalue)))

(fn InterfaceScanner
  (bind _mesh (Variables|Character|GetMesh))
  (bind _returnvalue (Transformation|GetSocketLocation _mesh "head"))
  (bind (_outhit _returnvalue_2) (Collision|SphereTraceByChannel _returnvalue (+ _returnvalue (* (Math|Vector|Normalize (- (Variables|Default|GetLookAtPoint) _returnvalue)) 2e+02)) 3e+01 "TraceTypeQuery3" false 0 "ForOneFrame"))
  (if _returnvalue_2
    (return (.HitActor (Collision|BreakHitResult _outhit)))))

(fn GetWeaponSlot
  (bind _weaponslots (Variables|Default|GetWeaponSlots))
  (bind _weaponslotsindex (Variables|Default|GetWeaponSlotsIndex))
  (bind _output (Utilities|Array|Get(acopy) _weaponslots _weaponslotsindex))
  (return (.weaponbase _output) (.weapontype _output) (.holster _output)))

(fn GetCurrentWeaponSlot
  (bind _weaponslots (Variables|Default|GetWeaponSlots))
  (bind _currentweaponslotsindex (Variables|Default|GetCurrentWeaponSlotsIndex))
  (bind _output (Utilities|Array|Get(acopy) _weaponslots _currentweaponslotsindex))
  (return (.weaponbase _output) (.weapontype _output) (.holster _output)))

(fn MontageIsNotRunning
  (return (== (Animation|Curves|GetCurveValue (Components|SkeletalMesh|GetAnimInstance (Variables|Character|GetMesh)) "MontageIsRunning") 0.0)))

(fn CloseWeaponLight
  (Default|CloseLight (.Weapon%20Base (CallFunction|GetCurrentWeaponSlot)))
  (Variables|Default|SetIsLightOpen false))

(fn OpenWeaponLight
  (Default|OpenLight (.Weapon%20Base (CallFunction|GetCurrentWeaponSlot)))
  (Variables|Default|SetIsLightOpen true))

(fn GetCurrentWeaponValue
  (bind _weapon_base (CallFunction|GetCurrentWeaponSlot))
  (if (!= _weapon_base 0)
    (bind _weaponvalue (Class|BPIWeaponBase|SendValue(Message) _weapon_base))
    (Variables|Default|SetCurrentWeaponValue _weaponvalue)))

(fn SendCurrentWeaponValue
  (return (Variables|Default|GetCurrentWeaponValue) (Variables|Default|GetIsCombate)))

(fn SendValue
  (return (Utilities|Struct|MakeBPIS_SendValue (Variables|Default|GetYaw) (Variables|Default|GetPitch) (Variables|Default|GetDirction) (Variables|Default|GetSpeed) (Variables|Default|GetIsInAir) (Variables|Default|GetIsCombate) (Variables|Default|GetIsADS) (Variables|Default|GetUseLHandIK) (Variables|Default|GetGripLOfset) (Variables|Default|GetAim%20Baseline%20Offset) (.Weapon%20Type (CallFunction|GetCurrentWeaponSlot)) (Variables|Default|GetHp) (Variables|Default|GetMaxHp) (Variables|Default|GetStamina) (Variables|Default|GetMaxStamina))))