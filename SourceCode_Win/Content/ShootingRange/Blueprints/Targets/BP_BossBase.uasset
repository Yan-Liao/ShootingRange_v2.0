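; Base boss enemy for the shooting range: an AI-controlled target that moves, attacks and can be killed.
; BeginPlay fills the boss blackboard with the player and itself, while BossDebut notifies the boss controller.
; Move and attack events drive navigation and damage, with audio cues throughout.
; At zero health it drops its controller, releases ShapePlane to unconstrained physics and reports EnemyDown to the game state once.
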(event EventAttack
  (params (AttackWho :type Actor%20Object%20Reference))
  (Audio|Components|Audio|Play (Variables|Default|GetACHit) 0.0)
  (Game|Damage|ApplyDamage AttackWho (Variables|Default|GetDamage) 0 0))

(event EventBossDebut
  (bind _asbp_boss_controler (Utilities|Casting|CastToBP_BossControler (Pawn|GetController self)))
  (Default|BossComing _asbp_boss_controler)
  (Audio|Components|Audio|Play (Variables|Default|GetACTargetUp) 0.0))

(event EventMoveto
  (params (Target :type Actor%20Object%20Reference))
  (AI|Navigation|SimpleMovetoActor (AI|GetAIController self) Target))

(event EventBeginPlay
  (bind _self self)
  (bind _returnvalue (AI|GetBlackboard _self))
  (Class|AIController|UseBlackboard (AI|GetAIController _self) "/Game/ShootingRange/Blueprints/Targets/AI/BB_Boss.BB_Boss")
  (AI|Components|Blackboard|SetValueasObject _returnvalue (Variables|Default|GetFindWho) (Game|GetPlayerCharacter 0))
  (AI|Components|Blackboard|SetValueasObject _returnvalue (Variables|Default|GetSelfName) self))

(event Game|Damage|EventAnyDamage
  (params (Damage :type Float%20%28single-precision%29) (DamageType :type Damage%20Type%20Object%20Reference) (InstigatedBy :type Controller%20Object%20Reference) (DamageCauser :type Actor%20Object%20Reference))
  (Utilities|FlowControl|Sequence
    (:then_0
      (Audio|Components|Audio|Play (Variables|Default|GetACBeHit) 0.0))
    (:then_1
      (if (not (Variables|Default|GetTargetIsDown))
        (Development|PrintString "Hit")
        (bind _output_get (Variables|Default|SetTargetHp (Math|Float|Max(Float) (- (Variables|Default|GetTargetHp) Damage) 0.0)))
        (Development|PrintString (Utilities|String|ToString(Float) _output_get))
        (Math|Float|CompareFloat _output_get 0.0
          (:==
            _)
          (:<
            _))
        (Utilities|FlowControl|DoOnce false
          (:Completed
            (Class|Pawn|DetachfromControllerPendingDestroy)
            (Variables|Default|SetTargetIsDown true)
            (Physics|SetSimulatePhysics (Variables|Default|GetShape_Plane) true)
            (Class|PrimitiveComponent|SetConstraintMode (Variables|Default|GetShape_Plane) "None")
            (Audio|Components|Audio|Play (Variables|Default|GetACTargetDown) 0.0)
            (bind _asbp_my_game_state (Utilities|Casting|CastToBP_MyGameState (Game|GetGameState)))
            (Default|EnemyDown _asbp_my_game_state)))))))

(fn ConstructionScript)