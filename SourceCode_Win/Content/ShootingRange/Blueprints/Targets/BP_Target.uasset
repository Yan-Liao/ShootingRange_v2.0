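; BP_Target is a shooting range target that takes damage and goes down when its health runs out.
; Every hit plays the ACBeHit component, and while the target is up the damage lowers TargetHp, clamped at zero.
; At zero health it marks itself down once, releases the ShapePlane's constraint mode, and reports the kill to BP_MyGameState through EnemyDown.
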(event Game|Damage|EventAnyDamage
  (params (Damage :type Float%20%28single-precision%29) (DamageType :type Damage%20Type%20Object%20Reference) (InstigatedBy :type Controller%20Object%20Reference) (DamageCauser :type Actor%20Object%20Reference))
  (Utilities|FlowControl|Sequence
    (:then_0
      (Audio|Components|Audio|Play (Variables|Default|GetACBeHit) 0.0))
    (:then_1
      (if (not (Variables|Default|GetTargetIsDown))
        (bind _output_get (Variables|Default|SetTargetHp (Math|Float|Max(Float) (- (Variables|Default|GetTargetHp) Damage) 0.0)))
        (Math|Float|CompareFloat _output_get 0.0
          (:==
            _)
          (:<
            _))
        (Utilities|FlowControl|DoOnce false
          (:Completed
            (Variables|Default|SetTargetIsDown true)
            (Class|PrimitiveComponent|SetConstraintMode (Variables|Default|GetShape_Plane) "None")
            (bind _asbp_my_game_state (Utilities|Casting|CastToBP_MyGameState (Game|GetGameState)))
            (Default|EnemyDown _asbp_my_game_state)))))))

(fn ConstructionScript)