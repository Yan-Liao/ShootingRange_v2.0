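; BP_ProjectileBase is a projectile, by name the base for weapon projectiles in the shooting range, that damages and pushes what it hits.
; The StaticMesh hit event applies Damage to the other actor.
; If the hit component simulates physics, it adds an impulse at the hit location along the projectile's forward vector, scaled by Impulse.
; The projectile then destroys itself; the branch condition is fixed true.
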(event OnComponentHit(StaticMesh)
  (params (HitComponent :type Primitive%20Component%20Object%20Reference) (OtherActor :type Actor%20Object%20Reference) (OtherComp :type Primitive%20Component%20Object%20Reference) (NormalImpulse :type Vector :default "0, 0, 0") (Hit :type Hit%20Result%20Structure%20%28by%20ref%29))
  (bind (_bblockinghit _binitialoverlap _time _distance _location _impactpoint _normal _impactnormal _physmat _hitactor _hitcomponent) (Collision|BreakHitResult Hit))
  (if true
    (Game|Damage|ApplyDamage OtherActor (Variables|Default|GetDamage) 0 0)
    (if (Physics|IsSimulatingPhysics _hitcomponent "None")
      (Physics|AddImpulseatLocation _hitcomponent (* (Math|Vector|GetForwardVector (Transformation|GetActorRotation self)) (Variables|Default|GetImpulse)) _location "None"))
    (Actor|DestroyActor)
    (else
      (Actor|DestroyActor))))

(event EventBeginPlay)

(event Collision|EventActorBeginOverlap
  (params (OtherActor :type Actor%20Object%20Reference)))

(event EventTick
  (params (DeltaSeconds :type Float%20%28single-precision%29)))

(fn ConstructionScript)