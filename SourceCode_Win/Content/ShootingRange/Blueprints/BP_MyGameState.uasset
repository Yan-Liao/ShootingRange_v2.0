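; Game state for the shooting range that tracks the mission countdown, kill count and win or fail outcome.
; A timeline played in reverse drives the countdown, flagging low time at a threshold and failing the mission at zero.
; Failure pauses the game, shows the cursor and opens a fail widget, while success opens its own widget.
; SendValue exposes fail type, time, kills and low-time flag.
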(event EventCountTimeDown
  (bind _新建轨道_0 (Timeline|时间轴_0 ReverseFromEnd)
    (:Update
      (if (not (or (Variables|Default|GetIsMissionFailed) (Variables|Default|GetIsMissionSucceed)))
        (bind _output_get (Variables|Default|SetCountDownTime _新建轨道_0))
        (Math|Float|CompareFloat _output_get (Variables|Default|GetLessTime)
          (:==
            _)
          (:<
            _))
        (Utilities|FlowControl|Sequence
          (:then_0
            (Utilities|FlowControl|DoOnce false
              (:Completed
                (Variables|Default|SetTimeIsLess true))))
          (:then_1
            (Math|Float|CompareFloat _output_get 0.0
              (:==
                _)
              (:<
                _))
            (Utilities|FlowControl|DoOnce false
              (:Completed
                (CallFunction|MissionFailed "NewEnumerator1")))))))))

(event EventEnemyDown
  (Math|Integer|IncrementInt (Variables|Default|GetKillTargetNum)))

(event EventMissionFailed
  (params (FailType :type EFailType%20Enum :default "NewEnumerator0"))
  (Utilities|FlowControl|DoOnce false
    (:Completed
      (Variables|Default|SetFailType FailType)
      (Variables|Default|SetIsMissionFailed true)
      (Game|SetGamePaused true)
      (Variables|/Script/Engine.PlayerController|SetbShowMouseCursor (Game|GetPlayerController 0) true)
      (bind _returnvalue (UserInterface|CreateWidget "/Game/ShootingRange/UI/WBP_Fail.WBP_Fail_C"))
      (UserInterface|Viewport|AddtoViewport _returnvalue 0))))

(event EventMissionSucceed
  (Utilities|FlowControl|DoOnce false
    (:Completed
      (Variables|Default|SetIsMissionSucceed true)
      (bind _returnvalue (UserInterface|CreateWidget "/Game/ShootingRange/UI/WBP_Succeed.WBP_Succeed_C"))
      (UserInterface|Viewport|AddtoViewport _returnvalue 0))))

(fn ConstructionScript)

(fn SendValue
  (return (Utilities|Struct|MakeSGameStateValue (Variables|Default|GetFailType) (Variables|Default|GetCountDownTime) (Variables|Default|GetKillTargetNum) (Variables|Default|GetTimeIsLess))))